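; EnemySpawner is an actor Blueprint that spawns Enemy_Character AI pawns within its SpawnVolume box.
; Its SpawnEnemy event counts every Enemy_Character in the level and spawns one more at a random point in the box while the count is below MaxEnemies.
; Nothing in this Blueprint calls SpawnEnemy, and BeginPlay, overlap and Tick are unused stubs.
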(event Custom|SpawnEnemy
  (bind _outactors (Actor|GetAllActorsOfClass "/Game/Blueprints/Enemy_Character.Enemy_Character_C"))
  (if (< (Utilities|Array|Length _outactors) (Variables|Default|GetMaxEnemies))
    (AI|SpawnAIFromClass "/Game/Blueprints/Enemy_Character.Enemy_Character_C" 0 (Math|Random|RandomPointinBoundingBox (Transformation|GetWorldLocation (Variables|Default|GetSpawnVolume)) (Components|Box|GetScaledBoxExtent (Variables|Default|GetSpawnVolume))) "0, 0, 0" false 0)))

(event EventBeginPlay)

(event Collision|EventActorBeginOverlap
  (params (OtherActor :type Actor%20Object%20Reference)))

(event EventTick
  (params (DeltaSeconds :type Float%20%28single-precision%29)))

(fn ConstructionScript)